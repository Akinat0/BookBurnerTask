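; Manager for a turn-based tactical duel that spawns the player and AI opponent from game instance data and creates the fight canvas.
; Cycles preparation, fight and result phases, using AIMoveTo with MultiGates to wait for both fighters to approach and return.
; Both attack each round, dealing damage unless the attack position matches the defender's defense position.
; The loop repeats until someone dies; restart and exit load levels.
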(event `self.ReceiveBeginPlay`
  (bind _asbp_tactic_game_instance (cast `/Game/Blueprints/BP_TacticGameInstance` (`GameplayStatics.GetGameInstance`)))
  (bind (_gamedata_playerparams _gamedata_isfighting _gamedata_currentopponentparameters) (break `/Game/Blueprints/Struct_GameData` (`/Game/Blueprints/BP_TacticGameInstance.GameData` _asbp_tactic_game_instance)))
  (bind _returnvalue (`|SpawnActorFromClass` "/Game/TacticFight/Blueprints/Characters/BP_TacticFightCharacterPlayer.BP_TacticFightCharacterPlayer_C" (`self.GetTransform` (`self.PlayerPoint`)) "Undefined" "OverrideRootScale" null _gamedata_playerparams null))
  (set `self.PlayerCharacter` _returnvalue)
  (bind _returnvalue_2 (`|SpawnActorFromClass` "/Game/TacticFight/Blueprints/Characters/BP_TacticFightCharacterAI.BP_TacticFightCharacterAI_C" (`self.GetTransform` (`self.OpponentPoint`)) "Undefined" "OverrideRootScale" null _gamedata_currentopponentparameters null))
  (set `self.OpponentCharacter` _returnvalue_2)
  (bind _returnvalue_3 (`|CreateWidget` "/Game/TacticFight/Blueprints/UI/W_TacticFightCanvas.W_TacticFightCanvas_C"))
  (bind _output_get (set `self.Canvas` _returnvalue_3))
  (`/Game/TacticFight/Blueprints/UI/W_TacticFightCanvas.Initialize` _output_get self (`self.PlayerCharacter`) (`self.OpponentCharacter`))
  (`UserWidget.AddToViewport` (`self.Canvas`) 0)
  (`self.StartPreparationPhase`))

(event `StartPreparationPhase`
  (set `self.Phase` "NewEnumerator1")
  (`/Game/TacticFight/Blueprints/Characters/BP_TacticFightCharacterBase.MakeDecision` (`self.PlayerCharacter`))
  (`/Game/TacticFight/Blueprints/Characters/BP_TacticFightCharacterBase.MakeDecision` (`self.OpponentCharacter`)))

(event `StartFightPhase`
  (if (and (`|EnumEquality` (`self.Phase`) "NewEnumerator1") (`/Game/TacticFight/Blueprints/Characters/BP_TacticFightCharacterBase.GetDecision` (`self.PlayerCharacter`)) (`/Game/TacticFight/Blueprints/Characters/BP_TacticFightCharacterBase.GetDecision` (`self.OpponentCharacter`)))
    (set `self.Phase` "NewEnumerator2")
    (`self.SetFocusPoints`)
    (`|AIMoveTo` (`self.PlayerCharacter`) (0.0 0.0 0.0) (`self.FightPoint`)
      (:`then`
        (`|AIMoveTo` (`self.OpponentCharacter`) (0.0 0.0 0.0) (`self.FightPoint`) 120.0
          (:`OnSuccess`
            _)))
      (:`OnSuccess`
        _))
    ;[1 1 1] Wait for both tasks
    (`|MultiGate` false :!label _label
      (:`Out 1`
        (`|ExecutionSequence`
          (:`then_0`
            (goto _label :!via `Reset`))
          (:`then_1`
            (`self.Process Fight`)
            (`/Game/TacticFight/Blueprints/Characters/BP_TacticFightCharacterBase.Clean Decision` (`self.PlayerCharacter`))
            (`/Game/TacticFight/Blueprints/Characters/BP_TacticFightCharacterBase.Clean Decision` (`self.OpponentCharacter`))
            (`/Game/TacticFight/Blueprints/UI/W_TacticFightCanvas.CleanSelectedDecision` (`self.Canvas`))
            (`KismetSystemLibrary.Delay` 1.0)
            (`self.StartResultPhase`)))))))

(event `StartResultPhase`
  (bind _result (`self.GetResult`))
  (set `self.Phase` "NewEnumerator3")
  (`self.ClearFocusPoints`)
  (`|AIMoveTo` (`self.PlayerCharacter`) (`KismetMathLibrary.SelectVector` (`self.K2_GetActorLocation` (`self.PlayerCharacter`)) (`self.K2_GetActorLocation` (`self.PlayerPoint`)) (`/Game/TacticFight/Blueprints/Characters/BP_TacticFightCharacterBase.IsDead` (`self.PlayerCharacter`))) null
    (:`then`
      (`|AIMoveTo` (`self.OpponentCharacter`) (`KismetMathLibrary.SelectVector` (`self.K2_GetActorLocation` (`self.OpponentCharacter`)) (`self.K2_GetActorLocation` (`self.OpponentPoint`)) (`/Game/TacticFight/Blueprints/Characters/BP_TacticFightCharacterBase.IsDead` (`self.OpponentCharacter`))) null 100.0
        (:`OnSuccess`
          _)))
    (:`OnSuccess`
      _))
  ;[1 1 1] Wait for both tasks
  (`|MultiGate` false :!label _label_2
    (:`Out 1`
      (`|ExecutionSequence`
        (:`then_0`
          (goto _label_2 :!via `Reset`))
        (:`then_1`
          (`self.SetFocusPoints`)
          (`/Game/TacticFight/Blueprints/UI/W_TacticFightCanvas.SetResult` (`self.Canvas`) _result)
          (if (`|EnumEquality` _result "NewEnumerator0")
            (`self.StartPreparationPhase`)))))))

(event `Restart`
  (bind _returnvalue (`GameplayStatics.GetCurrentLevelName` true))
  (`GameplayStatics.OpenLevel` (`KismetStringLibrary.Conv_StringToName` _returnvalue)))

(event `Exit`
  (`GameplayStatics.OpenLevelBySoftObjectPtr` "/Game/TopDown/Maps/TopDownMap.TopDownMap"))

(fn `Attack`
  (params (Attacker :type "/Game/TacticFight/Blueprints/Characters/BP_TacticFightCharacterBase Object Reference") (Defender :type "/Game/TacticFight/Blueprints/Characters/BP_TacticFightCharacterBase Object Reference"))
  (returns (Result :type "/Game/TacticFight/Blueprints/Struct_TacticFightAttackResult Structure"))
  (bind (_params_name _params_damage) (break `/Game/TacticFight/Blueprints/Struct_TacticFightCharacterParameters` (`/Game/TacticFight/Blueprints/Characters/BP_TacticFightCharacterBase.Params` (`local.Attacker`))))
  (if (`self.IsSuccessAttack` (`.AttackPosition_7_1E58070D4C460CC09075BFAD776A0B76` (break `/Game/TacticFight/Blueprints/Struct_TacticFightDecision` (`.Decision` (`/Game/TacticFight/Blueprints/Characters/BP_TacticFightCharacterBase.GetDecision` Attacker)))) (break `/Game/TacticFight/Blueprints/Struct_TacticFightDecision` (`.Decision` (`/Game/TacticFight/Blueprints/Characters/BP_TacticFightCharacterBase.GetDecision` Defender))))
    (`/Game/TacticFight/Blueprints/Characters/BP_TacticFightCharacterBase.DealDamage` (`local.Defender`) _params_damage)
    (return (make `/Game/TacticFight/Blueprints/Struct_TacticFightAttackResult` false _params_damage))
    (else
      (return (make `/Game/TacticFight/Blueprints/Struct_TacticFightAttackResult` true)))))

(fn `ClearFocusPoints`
  (`|ExecutionSequence`
    (:`then_0`
      (bind _asaicontroller (cast `AIController` (`Pawn.GetController` (`self.OpponentCharacter`))))
      (`AIController.K2_ClearFocus` _asaicontroller))
    (:`then_1`
      (bind _asaicontroller_2 (cast `AIController` (`Pawn.GetController` (`self.PlayerCharacter`))))
      (`AIController.K2_ClearFocus` _asaicontroller_2))))

(fn `GetPhase`
  (returns (Phase :type "/Game/TacticFight/Blueprints/E_TacticFightPhase Enum"))
  (return (`self.Phase`)))

(fn `GetResult`
  (returns (Result :type "/Game/TacticFight/Blueprints/E_TacticFightResult Enum"))
  (locals (IsPlayerDead :type Boolean :default false) (IsOpponentDead :type Boolean :default false))
  (set `local.IsPlayerDead` (`/Game/TacticFight/Blueprints/Characters/BP_TacticFightCharacterBase.IsDead` (`self.PlayerCharacter`)))
  (set `local.IsOpponentDead` (`/Game/TacticFight/Blueprints/Characters/BP_TacticFightCharacterBase.IsDead` (`self.OpponentCharacter`)))
  (if (and (`local.IsPlayerDead`) (`local.IsOpponentDead`))
    (return "NewEnumerator3")
    (elif (and (not (`local.IsPlayerDead`)) (`local.IsOpponentDead`))
      (return "NewEnumerator1")
      (elif (and (`local.IsPlayerDead`) (not (`local.IsOpponentDead`)))
        (return "NewEnumerator2")
        (else
          (return "NewEnumerator0"))))))

(fn `IsSuccessAttack`
  (params (AttackPosition :type "/Game/TacticFight/Blueprints/E_TacticFightPositionType Enum" :default "NewEnumerator0") (DefensePosition :type "/Game/TacticFight/Blueprints/E_TacticFightPositionType Enum" :default "NewEnumerator0"))
  (returns (IsSuccess :type Boolean))
  (return (`|EnumInequality` AttackPosition DefensePosition)))

(fn `PrintDecision`
  (params (Name :type Text) (Decision :type "/Game/TacticFight/Blueprints/Struct_TacticFightDecision Structure"))
  (`KismetSystemLibrary.PrintString` (`KismetStringLibrary.Concat_StrStr` (`KismetTextLibrary.Conv_TextToString` Name) " Def: " (`|GetEnumeratorNameAsString` Decision_DefensePosition_6_B1081EE04F3F84793257E08F40973B9A) " Attack: " (`|GetEnumeratorNameAsString` Decision_AttackPosition_7_1E58070D4C460CC09075BFAD776A0B76))))

(fn `Process Fight`
  (bind _opponentcharacter (`self.OpponentCharacter`))
  (bind _playercharacter (`self.PlayerCharacter`))
  (bind _result (`self.Attack` (`self.PlayerCharacter`) _opponentcharacter))
  (`/Game/TacticFight/Blueprints/UI/W_TacticFightCanvas.ShowAttackResult` (`self.Canvas`) _opponentcharacter _result)
  (bind _result_2 (`self.Attack` (`self.OpponentCharacter`) _playercharacter))
  (`/Game/TacticFight/Blueprints/UI/W_TacticFightCanvas.ShowAttackResult` (`self.Canvas`) _playercharacter _result_2))

(fn `SetFocusPoints`
  (`|ExecutionSequence`
    (:`then_0`
      (bind _asaicontroller (cast `AIController` (`Pawn.GetController` (`self.OpponentCharacter`))))
      (`AIController.K2_SetFocus` _asaicontroller (`self.PlayerCharacter`)))
    (:`then_1`
      (bind _asaicontroller_2 (cast `AIController` (`Pawn.GetController` (`self.PlayerCharacter`))))
      (`AIController.K2_SetFocus` _asaicontroller_2 (`self.OpponentCharacter`)))))

(fn `UserConstructionScript`)