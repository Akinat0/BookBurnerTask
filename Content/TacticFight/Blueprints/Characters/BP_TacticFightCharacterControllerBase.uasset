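; Base character controller for TacticFight that produces a fight decision made of a defense position and an attack position.
; GetDecision calls GetRandomPositionType separately for each position, picking uniformly among three position types and returning both in a TacticFightDecision struct.
; BeginPlay seeds RandomStream with a fixed value, but the picks use the global RandomInteger, so that seed does not affect them.
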(event `self.ReceiveBeginPlay`
  (`KismetMathLibrary.SetRandomStreamSeed` (`self.RandomStream`)))

(fn `GetDecision`
  (returns (Decision :type "/Game/TacticFight/Blueprints/Struct_TacticFightDecision Structure"))
  (bind _position (`self.GetRandomPositionType`))
  (bind _position_2 (`self.GetRandomPositionType`))
  (return (make `/Game/TacticFight/Blueprints/Struct_TacticFightDecision` _position _position_2)))

(fn `GetRandomPositionType`
  (returns (Position :type "/Game/TacticFight/Blueprints/E_TacticFightPositionType Enum"))
  (return (select `int` (`KismetMathLibrary.RandomInteger` 3) :`0` "NewEnumerator1" :`1` "NewEnumerator2" :`2` "NewEnumerator3" :!type "/Game/TacticFight/Blueprints/E_TacticFightPositionType Enum")))

(fn `UserConstructionScript`)