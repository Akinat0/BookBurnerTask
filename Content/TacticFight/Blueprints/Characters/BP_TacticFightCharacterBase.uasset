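; Base character Blueprint for the TacticFight game, holding a fighter's HP and its chosen attack and defense positions.
; HP starts from Params.HP on BeginPlay, and DealDamage clamps it between zero and that maximum, with IsDead true at zero.
; MakeDecision is an empty stub, while GetDecision reports the Decision as ready once both positions leave their default enum value.
; CleanDecision resets the stored choice.
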(event `self.ReceiveBeginPlay`
  (bind (_params_name _params_damage _params_hp) (break `/Game/TacticFight/Blueprints/Struct_TacticFightCharacterParameters` (`self.Params`)))
  (set `self.HP` _params_hp))

(fn `Clean Decision`
  (set `self.Decision` (struct)))

(fn `DealDamage`
  (params (Damage :type "Float (double-precision)"))
  (bind (_params_name _params_damage _params_hp) (break `/Game/TacticFight/Blueprints/Struct_TacticFightCharacterParameters` (`self.Params`)))
  (set `self.HP` (`KismetMathLibrary.FClamp` (- (`self.HP`) Damage) 0.0 _params_hp)))

(fn `GetDecision`
  (returns (IsReady :type Boolean) (Decision :type "/Game/TacticFight/Blueprints/Struct_TacticFightDecision Structure"))
  (bind (_defenseposition _attackposition) (break `/Game/TacticFight/Blueprints/Struct_TacticFightDecision` (`self.Decision`)))
  (return (and (`|EnumInequality` _defenseposition "NewEnumerator0") (`|EnumInequality` _attackposition "NewEnumerator0")) (`self.Decision`)))

(fn `GetHP`
  (returns (HP :type "Float (double-precision)"))
  (return (`self.HP`)))

(fn `IsDead`
  (returns (IsDead :type Boolean))
  (return (<= (`self.HP`) 0.0)))

(fn `MakeDecision`)

(fn `UserConstructionScript`)